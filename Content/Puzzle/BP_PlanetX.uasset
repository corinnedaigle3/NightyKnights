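; BP_PlanetX is a puzzle actor that travels along the Spline_X actor found in the level at BeginPlay.
; Pressing key 9 flip-flops between playing and stopping a timeline, with play rate set from TimeToComplete.
; Each timeline update maps its Move value to a distance along the spline and applies that point's world location and rotation to the actor.
; The MoveObj event called at BeginPlay is empty.
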(event Custom|Move%20Obj)

(event EventBeginPlay
  (bind _returnvalue (Actor|GetActorOfClass "/Game/Puzzle/Spline_X.Spline_X_C"))
  (Variables|Default|SetSpline%20REF _returnvalue)
  (CallFunction|MoveObj))

(event Input|KeyboardEvents|9
  (params (Key :type Key%20Structure :default "None"))
  (bind _spline_ref (Variables|Default|GetSpline%20REF))
  (bind _spline (Variables|/Game/Puzzle/Spline_X.Spline_X_C|GetSpline _spline_ref))
  (:Pressed
    (Components|Timeline|SetPlayRate (Variables|Default|GetMove%20Obj%20Timeline) (/ 1.0 (Variables|Default|GetTimeToComplete)))
    (Utilities|FlowControl|FlipFlop
      (:A
        (bind _move (Timeline|Move%20Obj%20Timeline Play)
          (:Update
            (Transformation|SetActorTransform (Math|Transform|MakeTransform (Spline|GetLocationatDistanceAlongSpline _spline (Math|Float|Lerp 0.0 (Spline|GetSplineLength (Variables|/Game/Puzzle/Spline_X.Spline_X_C|GetSpline (Variables|Default|GetSpline%20REF))) _move) "World") (Spline|GetRotationatDistanceAlongSpline _spline (Math|Float|Lerp 0.0 (Spline|GetSplineLength (Variables|/Game/Puzzle/Spline_X.Spline_X_C|GetSpline (Variables|Default|GetSpline%20REF))) _move) "World") "1.000000,1.000000,1.000000")))))
      (:B
        (Timeline|Move%20Obj%20Timeline Stop)))))

(fn ConstructionScript)